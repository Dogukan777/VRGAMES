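; Interactive standing lamp prop that the player toggles on and off with the E key while inside its trigger box.
; Trigger box overlap enables and disables input on the actor for player controller 0.
; The ON timeline plays or reverses based on IsOn, animating the point light intensity and an emissive strength parameter on a dynamic material created for the mesh at BeginPlay.
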(event OnComponentBeginOverlap(TriggerBoxR)
  (params (OverlappedComponent :type Primitive%20Component%20Object%20Reference) (OtherActor :type Actor%20Object%20Reference) (OtherComp :type Primitive%20Component%20Object%20Reference) (OtherBodyIndex :type Integer) (bFromSweep :type Boolean) (SweepResult :type Hit%20Result%20Structure%20%28by%20ref%29))
  (Input|EnableInput (Game|GetPlayerController 0)))

(event OnComponentEndOverlap(TriggerBoxR)
  (params (OverlappedComponent :type Primitive%20Component%20Object%20Reference) (OtherActor :type Actor%20Object%20Reference) (OtherComp :type Primitive%20Component%20Object%20Reference) (OtherBodyIndex :type Integer))
  (Input|DisableInput (Game|GetPlayerController 0)))

(event EventBeginPlay
  (bind _returnvalue (Rendering|Material|CreateDynamicMaterialInstance (Variables|Default|GetSM_StandLighting) 1 0 "Stand_Lighting_EM_Strength" :!class /Script/Engine.PrimitiveComponent))
  (Variables|Default|SetMat _returnvalue))

(event Collision|EventActorBeginOverlap
  (params (OtherActor :type Actor%20Object%20Reference)))

(event EventTick
  (params (DeltaSeconds :type Float%20%28single-precision%29)))

(event Input|KeyboardEvents|E
  (params (Key :type Key%20Structure))
  (:Pressed
    (if (Variables|Default|GetIsOn)
      (Variables|Default|SetIsOn false)
      (bind (_direction _on _intencity) (Timeline|ON Reverse)
        (:Update
          (Rendering|Material|SetScalarParameterValue (Variables|Default|GetMat) "Stand_Lighting_EM_Strength" _on :!class /Script/Engine.MaterialInstanceDynamic)
          (Rendering|Components|Light|SetIntensity (Variables|Default|GetPointLight) _intencity)))
      (else
        (Variables|Default|SetIsOn true)
        (Timeline|ON Play)))))

(fn ConstructionScript)