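; BP_Mirror_1 is an interactable mirror prop that toggles between flip and hide animations when E is pressed.
; TriggerBoxR enables player input on overlap and disables it when the overlap ends.
; The IsClose flag picks the next animation on SKMMirror, and presses are ignored while one is playing.
; Tick hides the UI component during animation playback and shows it otherwise.
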(event OnComponentBeginOverlap(TriggerBoxR)
  (params (OverlappedComponent :type Primitive%20Component%20Object%20Reference) (OtherActor :type Actor%20Object%20Reference) (OtherComp :type Primitive%20Component%20Object%20Reference) (OtherBodyIndex :type Integer) (bFromSweep :type Boolean) (SweepResult :type Hit%20Result%20Structure%20%28by%20ref%29))
  (Input|EnableInput (Game|GetPlayerController 0)))

(event OnComponentEndOverlap(TriggerBoxR)
  (params (OverlappedComponent :type Primitive%20Component%20Object%20Reference) (OtherActor :type Actor%20Object%20Reference) (OtherComp :type Primitive%20Component%20Object%20Reference) (OtherBodyIndex :type Integer))
  (Input|DisableInput (Game|GetPlayerController 0)))

(event EventBeginPlay)

(event Collision|EventActorBeginOverlap
  (params (OtherActor :type Actor%20Object%20Reference)))

(event EventTick
  (params (DeltaSeconds :type Float%20%28single-precision%29))
  (if (Audio|Components|Audio|IsPlaying (Variables|Default|GetSKM_Mirror))
    (CallFunction|SetUI true)
    (else
      (CallFunction|SetUI false))))

(event Input|KeyboardEvents|E
  (params (Key :type Key%20Structure))
  (bind _skm_mirror (Variables|Default|GetSKM_Mirror))
  (:Pressed
    (if (not (Audio|Components|Audio|IsPlaying _skm_mirror))
      (if (Variables|Default|GetIsClose)
        (Components|Animation|PlayAnimation _skm_mirror "/Game/KTInteractionPropVol2/Animation/ANIM_Mirror_Flip.ANIM_Mirror_Flip" false)
        (Variables|Default|SetIsClose false)
        (else
          (Components|Animation|PlayAnimation _skm_mirror "/Game/KTInteractionPropVol2/Animation/ANIM_Mirror_Hide.ANIM_Mirror_Hide" false)
          (Variables|Default|SetIsClose true))))))

(fn ConstructionScript)

(fn SetUI
  (params (Hidden :type Boolean))
  (Development|SetHiddeninGame (Variables|Default|GetUI) Hidden false))